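; VR player pawn for Pong: a full-body avatar with hand-attached meshes showing the saved paddle.
; Outside setup mode, BeginPlay sizes the Ynnk VR avatar from GameInstance calibration, attaches hand meshes to skeleton sockets and loads saved customization.
; Enhanced Input drives ball recall to either hand, test game start, and a spawned pause menu that toggles target-mode pause.
; Right grip applies the selected body mesh and saves it to the customization slot.
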(event Input|EnhancedActionEvents|EnhancedInputActionIA_TestAction
  (params (ActionValue :type Boolean) (ElapsedSeconds :type Float%20%28double-precision%29) (TriggeredSeconds :type Float%20%28double-precision%29) (InputAction :type Input%20Action%20Object%20Reference :default "/Game/VRPong/Input/Actions/IA_TestAction.IA_TestAction"))
  (bind _asbp_target_game_mode (Utilities|Casting|CastToBP_TargetGameMode (Game|GetGameMode)))
  (Class|TargetGameMode|StartGame _asbp_target_game_mode))

(event Input|EnhancedActionEvents|EnhancedInputActionIA_Pause
  (params (ActionValue :type Boolean) (ElapsedSeconds :type Float%20%28double-precision%29) (TriggeredSeconds :type Float%20%28double-precision%29) (InputAction :type Input%20Action%20Object%20Reference :default "/Game/VRPong/Input/Actions/IA_Pause.IA_Pause"))
  ;[1 1 1] Pause - Pause menu
  (:Started
    (Utilities|IsValid (Variables|Default|GetMenu%20Ref)
      (:Is%20Valid
        (CallFunction|CloseMenu)
        (Audio|PlaySound2D "/Game/VRPong/Sounds/Cues/SC_SFX_Dismiss-Menu.SC_SFX_Dismiss-Menu" 1.0 1.0 0.0 0 0))
      (:Is%20Not%20Valid
        (CallFunction|OpenMenu)
        (Audio|PlaySound2D "/Game/VRPong/Sounds/Cues/SC_SFX_Summon-Menu.SC_SFX_Summon-Menu" 1.0 1.0 0.0 0 0)))
    (bind _asbp_target_game_mode (Utilities|Casting|CastToBP_TargetGameMode (Game|GetGameMode)))
    (Default|TogglePause _asbp_target_game_mode)))

(event Input|EnhancedActionEvents|EnhancedInputActionIA_Interact_Left
  (params (ActionValue :type Boolean) (ElapsedSeconds :type Float%20%28double-precision%29) (TriggeredSeconds :type Float%20%28double-precision%29) (InputAction :type Input%20Action%20Object%20Reference :default "/Game/VRPong/Input/Actions/IA_Interact_Left.IA_Interact_Left"))
  (Class|VRPawn|RecallBalltoLeftHand))

(event Input|EnhancedActionEvents|EnhancedInputActionIA_Interact_Right
  (params (ActionValue :type Boolean) (ElapsedSeconds :type Float%20%28double-precision%29) (TriggeredSeconds :type Float%20%28double-precision%29) (InputAction :type Input%20Action%20Object%20Reference :default "/Game/VRPong/Input/Actions/IA_Interact_Right.IA_Interact_Right"))
  (Class|VRPawn|RecallBalltoRightHand))

(event Input|EnhancedActionEvents|EnhancedInputActionIA_Grip_Right
  (params (ActionValue :type Boolean) (ElapsedSeconds :type Float%20%28double-precision%29) (TriggeredSeconds :type Float%20%28double-precision%29) (InputAction :type Input%20Action%20Object%20Reference :default "/Game/VRPong/Input/Actions/IA_Grip_Right.IA_Grip_Right"))
  (bind _selectedmesh (Variables|Default|GetSelectedMesh))
  (bind _skeletal_mesh (Variables|/Game/VRPong/Blueprints/Interactable.Interactable_C|GetSkeletal%20Mesh _selectedmesh))
  (Utilities|IsValid _selectedmesh
    (:Is%20Valid
      (Utilities|IsValid _skeletal_mesh
        (:Is%20Valid
          (Components|SkeletalMesh|SetSkeletalMeshAsset (Variables|Character|GetMesh) _skeletal_mesh)
          (bind _returnvalue (SaveGame|CreateSaveGameObject "/Game/VRPong/Blueprints/SaveObjects/BP_PlayerSaveData.BP_PlayerSaveData_C"))
          (Variables|/Game/VRPong/Blueprints/SaveObjects/BP_PlayerSaveData.BP_PlayerSaveData_C|SetBodyMesh _returnvalue (Variables|/Script/Engine.SkeletalMeshComponent|GetSkeletalMeshAsset (Variables|Character|GetMesh)))
          (SaveGame|SaveGametoSlot _returnvalue "PlayerCustomization"))))))

(event EventBeginPlay
  (Utilities|Casting|CastToBP_SetupMode (Game|GetGameMode)
    (:CastFailed
      (Class|HeadMountedDisplayFunctionLibrary|SetTrackingOrigin "Stage")
      (Development|ExecuteConsoleCommand "vr.PixelDensity 1.0" 0)
      (CallFunction|InitializeYnnkComponent (Variables|Default|GetYnnkVrAvatar))
      (bind _asplayer_controller (Utilities|Casting|CastToPlayerController (Pawn|GetController)))
      (Utilities|Casting|CastToMenuGameMode (Game|GetGameMode)
        (:then
          _)
        (:CastFailed
          (Input|AddMappingContext (PlayerController|LocalPlayerSubsystems|GetEnhancedInputLocalPlayerSubsystem _asplayer_controller) "/Game/VRPong/Input/Contexts/IMC_DefaultPong.IMC_DefaultPong" 0 "(bIgnoreAllPressedKeysUntilRelease=True,bForceImmediately=False,bNotifyUserSettings=False)")))
      (Transformation|AttachComponentToComponent (Variables|Default|GetRightHandMesh) (Variables|Character|GetMesh) "Right Hand Socket" "SnapToTarget" "SnapToTarget" "KeepWorld" false)
      (Transformation|AttachComponentToComponent (Variables|Default|GetLeftHandMesh) (Variables|Character|GetMesh) "Left Hand Socket" "SnapToTarget" "SnapToTarget" "KeepWorld" false)
      (CallFunction|ApplySavedCustomization "PlayerCustomization"))))

(fn ConstructionScript)

(fn OpenMenu
  (bind _returnvalue (Game|SpawnActorfromClass "/Game/VRPong/Blueprints/ActorObjects/BP_Menu.BP_Menu_C" (Math|Transform|MakeTransform "0, 0, 0") "Undefined" "MultiplyWithRoot" 0 0))
  (Default|SetFirstMenu _returnvalue "Pause")
  (Variables|Default|SetMenu%20Ref _returnvalue))

(fn CloseMenu
  (bind _menu_ref (Variables|Default|GetMenu%20Ref))
  (Utilities|IsValid _menu_ref
    (:Is%20Valid
      (Actor|DestroyActor _menu_ref))))

(fn ApplySavedCustomization
  (params (Save%20Slot :type String))
  (bind _returnvalue (SaveGame|LoadGamefromSlot Save%20Slot))
  (bind _asbp_player_save_data (Utilities|Casting|CastToBP_PlayerSaveData _returnvalue))
  (Components|StaticMesh|SetStaticMesh (Variables|Default|GetLeftHandMesh) (Variables|/Game/VRPong/Blueprints/SaveObjects/BP_PlayerSaveData.BP_PlayerSaveData_C|GetPaddleMesh _asbp_player_save_data))
  (Components|StaticMesh|SetStaticMesh (Variables|Default|GetRightHandMesh) (Variables|/Game/VRPong/Blueprints/SaveObjects/BP_PlayerSaveData.BP_PlayerSaveData_C|GetPaddleMesh _asbp_player_save_data))
  (Components|SkeletalMesh|SetSkeletalMeshAsset (Variables|Character|GetMesh) (Variables|/Game/VRPong/Blueprints/SaveObjects/BP_PlayerSaveData.BP_PlayerSaveData_C|GetBodyMesh _asbp_player_save_data)))

(fn InitializeYnnkComponent
  (params (Avatar :type Ynnk%20Vr%20Avatar%20Component%20Object%20Reference))
  (bind _returnvalue (Class|YnnkVrAvatarComponent|Initialize Avatar))
  (if _returnvalue
    (bind _asbp_main_game_instance (Utilities|Casting|CastToBP_MainGameInstance (Game|GetGameInstance)))
    (Class|YnnkVrAvatarComponent|SetBodySizeManually Avatar (Variables|/Game/VRPong/Blueprints/Modes/BP_MainGameInstance.BP_MainGameInstance_C|GetStoredCalibration _asbp_main_game_instance) (Variables|/Game/VRPong/Blueprints/Modes/BP_MainGameInstance.BP_MainGameInstance_C|GetStoredCalibration _asbp_main_game_instance))
    (Class|YnnkVrAvatarComponent|SetEnabled Avatar true)
    (Actor|Tick|AddTickPrerequisiteActor Avatar self)))