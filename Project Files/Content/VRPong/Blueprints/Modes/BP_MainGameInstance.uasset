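; Game instance for VRPong that holds the player name and records high scores per level.
; UpdateRecordedScores loads or creates BP_HighScore saves in level-named "Global" and "Local" slots, updates both identically and saves them.
; CompareScores appends name-score pairs until ten exist, then inserts above the first lower score and trims the last.
; An in-memory session list keeps each level's best, returning whether the score set one.
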(event EventSaveLeaderboardValues
  (params (scores :type Array%20of%20String%20Int%20Pair%20Structures) (saveSlot :type String))
  (bind _returnvalue (SaveGame|CreateSaveGameObject "/Game/VRPong/Blueprints/SaveObjects/BP_HighScore.BP_HighScore_C"))
  (Variables|/Game/VRPong/Blueprints/SaveObjects/BP_HighScore.BP_HighScore_C|SetHighScore _returnvalue scores)
  (SaveGame|SaveGametoSlot _returnvalue saveSlot))

(fn SetPlayerName
  (params (Name :type String))
  (Variables|Default|SetPlayerName Name))

(fn UpdateRecordedScores
  (params (LevelName :type String) (Score :type Integer))
  (bind _returnvalue (Utilities|String|Append LevelName " Local"))
  (bind _returnvalue_2 (Utilities|String|Append LevelName " Global"))
  (Utilities|FlowControl|Sequence
    (:then_0
      (bind (_save_object _high_scores) (CallFunction|GetHighScores _returnvalue_2))
      (bind _updatedscores (CallFunction|CompareScores _high_scores Score))
      (Variables|/Game/VRPong/Blueprints/SaveObjects/BP_HighScore.BP_HighScore_C|SetHighScore _save_object _updatedscores)
      (SaveGame|SaveGametoSlot _save_object _returnvalue_2))
    (:then_1
      (bind (_save_object_2 _high_scores_2) (CallFunction|GetHighScores _returnvalue))
      (bind _updatedscores_2 (CallFunction|CompareScores _high_scores_2 Score))
      (Variables|/Game/VRPong/Blueprints/SaveObjects/BP_HighScore.BP_HighScore_C|SetHighScore _save_object_2 _updatedscores_2)
      (SaveGame|SaveGametoSlot _save_object_2 _returnvalue))
    (:then_2
      (if (Utilities|Array|IsEmpty (Variables|Default|GetsessionHighScores))
        (Utilities|Array|Add (Variables|Default|GetsessionHighScores) (Utilities|Struct|MakeStringIntPair LevelName Score))
        (return true)
        (else
          (bind (_array_element _array_index) (Utilities|Array|ForEachLoopwithBreak (Variables|Default|GetsessionHighScores) :!label _label)
            (:LoopBody
              (LocalVariables|SetStringIntPair _array_element)
              (if (Utilities|Enum|Equal(Enum) LevelName (.key (LocalVariables|GetStringIntPair)))
                (LocalVariables|SetLevelMatch true)
                (if (> Score (.value (LocalVariables|GetStringIntPair)))
                  (Utilities|Array|SetArrayElem (Variables|Default|GetsessionHighScores) _array_index (Utilities|Struct|MakeStringIntPair LevelName Score))
                  (LocalVariables|SetScoreRecorded true)
                  (goto _label Break))))
            (:Completed
              (if (LocalVariables|GetScoreRecorded)
                (LocalVariables|SetScoreRecorded false)
                (return true)
                (elif (LocalVariables|GetLevelMatch)
                  (LocalVariables|SetLevelMatch false)
                  (LocalVariables|SetScoreRecorded false)
                  (return false)
                  (else
                    (Utilities|Array|Add (Variables|Default|GetsessionHighScores) (Utilities|Struct|MakeStringIntPair LevelName Score))
                    (return true)))))))))))

(fn GetHighScores
  (params (Slot :type String))
  (bind _returnvalue (SaveGame|LoadGamefromSlot Slot))
  (bind _asbp_high_score (Utilities|Casting|CastToBP_HighScore _returnvalue)
    (:then
      (return _asbp_high_score (Variables|/Game/VRPong/Blueprints/SaveObjects/BP_HighScore.BP_HighScore_C|GetHighScore _asbp_high_score)))
    (:CastFailed
      (bind _returnvalue_2 (SaveGame|CreateSaveGameObject "/Game/VRPong/Blueprints/SaveObjects/BP_HighScore.BP_HighScore_C"))
      (return _returnvalue_2 (Variables|/Game/VRPong/Blueprints/SaveObjects/BP_HighScore.BP_HighScore_C|GetHighScore _returnvalue_2)))))

(fn CompareScores
  (params (SavedScores :type Array%20of%20String%20Int%20Pair%20Structures) (ScoreToQuery :type Integer))
  (if (== (Utilities|Array|Length SavedScores) 10)
    (bind (_array_element _array_index) (Utilities|Array|ForEachLoopwithBreak SavedScores :!label _label)
      (:LoopBody
        (bind _output_get (LocalVariables|SetTempStringIntPair _array_element))
        (if (> ScoreToQuery (.value _output_get))
          (Utilities|Array|Insert SavedScores (Utilities|Struct|MakeStringIntPair (Variables|Default|GetPlayerName) ScoreToQuery) _array_index)
          (Utilities|Array|RemoveIndex SavedScores 10)
          (goto _label Break)))
      (:Completed
        (return SavedScores)))
    (else
      (Utilities|Array|Add SavedScores (Utilities|Struct|MakeStringIntPair (Variables|Default|GetPlayerName) ScoreToQuery))
      (return SavedScores))))