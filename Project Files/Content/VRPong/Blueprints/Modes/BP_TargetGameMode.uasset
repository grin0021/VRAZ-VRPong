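; Game mode for target levels in VR Pong that applies the game instance's difficulty and reads the remaining match time.
; Its splash screen records the player's score, spawns a confetti actor ahead of the pawn to host the widget, enables confetti on high scores, and removes the Pong input mapping.
; Hiding it destroys that actor and restores input.
; Pause toggles global time dilation and a background audio low-pass.
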(event Custom|CountdownTImer
  (bind _returnvalue (Class|TargetGameMode|GetRemainingTime (Variables|Default|GetgameDurationHandle)))
  (Variables|Default|SetCountdown _returnvalue))

(event EventHideSplashScreen
  (bind _splashactor (Variables|Default|GetSplashActor))
  (Utilities|IsValid _splashactor
    (:Is%20Valid
      (Actor|DestroyActor _splashactor)
      (Input|AddMappingContext (PlayerController|LocalPlayerSubsystems|GetEnhancedInputLocalPlayerSubsystem (Game|GetPlayerController 0)) "/Game/VRPong/Input/Contexts/IMC_DefaultPong.IMC_DefaultPong" 0 "(bIgnoreAllPressedKeysUntilRelease=True,bForceImmediately=False,bNotifyUserSettings=False)")
      (Variables|Default|SetNewHighScore false))))

(event EventShowSplashScreen
  (bind _returnvalue (Game|Player|GetPlayerPawn 0))
  (bind _asbp_scoring_player_state (Utilities|Casting|CastToBP_ScoringPlayerState (Game|GetPlayerState 0)))
  (bind _returnvalue_2 (Class|ScoringPlayerState|PongGetScore _asbp_scoring_player_state))
  (bind _asbp_main_game_instance (Utilities|Casting|CastToBP_MainGameInstance (Game|GetGameInstance)))
  (bind _returnvalue_3 (Game|GetCurrentLevelName true))
  (bind _new_high_score (Default|UpdateRecordedScores _asbp_main_game_instance _returnvalue_3 _returnvalue_2))
  (Variables|Default|SetNewHighScore _new_high_score)
  (bind _returnvalue_4 (Game|SpawnActorfromClass "/Game/VRPong/Blueprints/ActorObjects/BP_Confetti.BP_Confetti_C" (Math|Transform|MakeTransform (+ (Transformation|GetActorLocation _returnvalue) (* (Transformation|GetActorForwardVector _returnvalue) 5e+01))) "Undefined" "MultiplyWithRoot" 0 (Variables|Default|GetNewHighScore) 0))
  (bind _aswb_splash_screen (Utilities|Casting|CastToWB_SplashScreen (Variables|Default|GetSplashScreen)))
  (Variables|/Game/VRPong/Blueprints/Widgets/WB_SplashScreen.WB_SplashScreen_C|SetNewHighScore _aswb_splash_screen (Variables|Default|GetNewHighScore))
  (UserInterface|SetWidget (Variables|/Game/VRPong/Blueprints/ActorObjects/BP_Menu.BP_Menu_C|GetWidget _returnvalue_4) (Variables|Default|GetSplashScreen))
  (Input|RemoveMappingContext (PlayerController|LocalPlayerSubsystems|GetEnhancedInputLocalPlayerSubsystem (Game|GetPlayerController 0)) "/Game/VRPong/Input/Contexts/IMC_DefaultPong.IMC_DefaultPong" "(bIgnoreAllPressedKeysUntilRelease=True,bForceImmediately=False,bNotifyUserSettings=False)")
  (Variables|Default|SetSplashActor _returnvalue_4))

(event EventBeginPlay
  (bind _asbp_main_game_instance (Utilities|Casting|CastToBP_MainGameInstance (Game|GetGameInstance)))
  (Class|TargetGameMode|SetDifficulty (Variables|/Game/VRPong/Blueprints/Modes/BP_MainGameInstance.BP_MainGameInstance_C|GetGameDifficulty _asbp_main_game_instance))
  (CallFunction|CountdownTImer))

(fn ConstructionScript)

(fn TogglePause
  (bind _output_get (Variables|Default|SetIsPaused (not (Variables|Default|GetIsPaused))))
  (if _output_get
    (Utilities|Time|SetGlobalTimeDilation 0.0)
    (else
      (Utilities|Time|SetGlobalTimeDilation 1.0)))
  (bind _outactors (Actor|GetAllActorsOfClass "/Game/VRPong/Blueprints/ActorMisc/BP_BackgroundAudio.BP_BackgroundAudio_C"))
  (for _array_element _outactors
    (Default|ToggleLowPass _array_element (Variables|Default|GetIsPaused))))

(fn IsGamePaused
  (return (Variables|Default|GetIsPaused)))