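; BP_Waypoint is a world waypoint actor whose widget component shows an objective marker, with off-screen direction indication.
; Each tick it turns toward the player camera and sets widget opacity from camera distance, so the marker fades up close.
; A screen-projection check swaps the widget between the actor and player camera through paired DoOnce gates.
; Off-screen, camera right/up dot products place the marker toward the waypoint within a safe viewport margin.
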(event EventBeginPlay
  (Variables|Default|SetplayerCamera (Game|GetPlayerCameraManager 0))
  (bind _aswb_objective_marker (Utilities|Casting|CastToWB_ObjectiveMarker (UserInterface|GetWidget (Variables|Default|GetWidget))))
  (Default|SetWaypoint _aswb_objective_marker (Variables|Default|GetWaypoint) self))

(event EventTick
  (params (DeltaSeconds :type Float%20%28single-precision%29))
  (bind _returnvalue (Transformation|GetActorLocation))
  (bind _returnvalue_2 (Game|GetPlayerCameraManager 0))
  (bind _returnvalue_3 (Camera|GetCameraLocation _returnvalue_2))
  (bind _returnvalue_4 (- _returnvalue_3 _returnvalue))
  (Transformation|SetActorRotation (Math|Rotator|FindLookatRotation _returnvalue _returnvalue_3))
  (Variables|Default|SetdirectionToCamera _returnvalue_4)
  (if (> 0.0 2.5e+02)
    (Widget|SetRenderOpacity (UserInterface|GetWidget (Variables|Default|GetWidget)) 1.0)
    (else
      (Widget|SetRenderOpacity (UserInterface|GetWidget (Variables|Default|GetWidget)) (/ (- (Math|Vector|VectorLength _returnvalue_4) 5e+01) (Math|Float|MakeLiteralFloat 2.5e+02)))))
  (CallFunction|SetWorldorViewPosition))

(fn ConstructionScript)

(fn SetWorldorViewPosition
  (bind _returnvalue (Game|GetPlayerController 0))
  (bind _returnvalue_2 (Transformation|GetActorLocation))
  (bind _returnvalue_3 (Viewport|GetViewportSize))
  (bind _halfviewport (LocalVariables|GethalfViewport))
  (bind _viewportsafety (LocalVariables|GetviewportSafety))
  (bind _screenposition (Class|GameplayStatics|ProjectWorldtoScreen _returnvalue _returnvalue_2 false))
  (bind _returnvalue_4 (* _halfviewport _viewportsafety))
  (bind (_x _y) (Math|Vector2D|BreakVector2D _screenposition))
  (bind _output_get (Variables|Default|SetinViewport (Math|Boolean|ANDBoolean (> _x 0.0) (< _x (.x _returnvalue_3)) (> _y 0.0) (< _y (.y _returnvalue_3)))))
  (if _output_get
    (Utilities|FlowControl|DoOnce false :!label _label
      (:Completed
        (Transformation|AttachComponentToComponent (Variables|Default|GetWidget) (Variables|Default|GetDefaultSceneRoot) "None" "SnapToTarget" "KeepRelative" "KeepRelative" false)
        (Transformation|SetRelativeLocationAndRotation (Variables|Default|GetWidget) "5.000000,6.000000,5.000000" "0, 0, 0" false false)
        (bind _aswb_objective_marker (Utilities|Casting|CastToWB_ObjectiveMarker (UserInterface|GetWidget (Variables|Default|GetWidget))))
        (Default|SetCanvasPosition _aswb_objective_marker (LocalVariables|GethalfViewport))
        (goto _label_2 Reset)))
    (else
      (Utilities|FlowControl|Sequence
        (:then_0
          (Utilities|FlowControl|DoOnce false :!label _label_2
            (:Completed
              (Transformation|AttachComponentToComponent (Variables|Default|GetWidget) (Actor|GetComponentbyClass (Game|GetPlayerCharacter 0) "/Script/Engine.CameraComponent") "None" "KeepRelative" "KeepRelative" "KeepRelative" false)
              (Transformation|SetRelativeLocationAndRotation (Variables|Default|GetWidget) "150.000000,0.000000,0.000000" "0.000000,180.000000,0.000000" false false)
              (goto _label Reset))))
        (:then_1
          (LocalVariables|SetScreenX (Math|Vector|DotProduct (Variables|Default|GetdirectionToCamera) (Math|Vector|GetRightVector (Variables|/Script/Engine.PlayerCameraManager|GetTransformComponent (Variables|Default|GetplayerCamera)))))
          (LocalVariables|SetScreenY (Math|Vector|DotProduct (Variables|Default|GetdirectionToCamera) (Math|Vector|GetUpVector (Variables|/Script/Engine.PlayerCameraManager|GetTransformComponent (Variables|Default|GetplayerCamera)))))
          (LocalVariables|SetScreen2D (Math|Vector2D|Normalize2D (Math|Vector2D|MakeVector2D (* (LocalVariables|GetScreenX) -1.0) (LocalVariables|GetScreenY))))
          (LocalVariables|SetwidgetScreenPos (+ _halfviewport (Math|Vector2D|MakeVector2D (* (.x _returnvalue_4) (.x (LocalVariables|GetScreen2D))) (* (.y (LocalVariables|GetScreen2D)) (.y _returnvalue_4)))))
          (bind _aswb_objective_marker_2 (Utilities|Casting|CastToWB_ObjectiveMarker (UserInterface|GetWidget (Variables|Default|GetWidget))))
          (Default|SetCanvasPosition _aswb_objective_marker_2 (LocalVariables|GetwidgetScreenPos)))))))