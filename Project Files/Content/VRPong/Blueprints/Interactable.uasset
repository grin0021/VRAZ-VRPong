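; Interactable is a component that highlights its owning actor and marks it as selected while the player is nearby in VRPong.
; On BeginPlay it caches the owner's static mesh and binds to the owner's capsule overlap events.
; Player overlap applies an overlay material and stores the component in BP_PlayPawn's SelectedMesh.
; Leaving clears both, then prints the selection's name for debugging.
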(event Custom|On%20Begin%20Overlap
  (params (OverlappedComponent :type Primitive%20Component%20Object%20Reference) (OtherActor :type Actor%20Object%20Reference) (OtherComp :type Primitive%20Component%20Object%20Reference) (OtherBodyIndex :type Integer) (bFromSweep :type Boolean) (SweepResult :type Hit%20Result%20Structure%20%28by%20ref%29))
  (bind _returnvalue (Game|GetPlayerCharacter 0))
  (if (== OtherActor _returnvalue)
    (Rendering|Material|SetOverlayMaterial (Variables|Default|GetOwning%20Mesh) (Variables|Default|GetOverlay%20Material) :!class /Script/Engine.MeshComponent)
    (bind _asbp_play_pawn (Utilities|Casting|CastToBP_PlayPawn _returnvalue))
    (Variables|/Game/VRPong/Blueprints/BP_PlayPawn.BP_PlayPawn_C|SetSelectedMesh _asbp_play_pawn self)))

(event Custom|On%20End%20Overlap
  (params (OverlappedComponent :type Primitive%20Component%20Object%20Reference) (OtherActor :type Actor%20Object%20Reference) (OtherComp :type Primitive%20Component%20Object%20Reference) (OtherBodyIndex :type Integer))
  (bind _returnvalue (Game|GetPlayerCharacter 0))
  (if (== OtherActor _returnvalue)
    (Rendering|Material|SetOverlayMaterial (Variables|Default|GetOwning%20Mesh) 0 :!class /Script/Engine.MeshComponent)
    (bind _asbp_play_pawn (Utilities|Casting|CastToBP_PlayPawn _returnvalue))
    (bind _output_get (Variables|/Game/VRPong/Blueprints/BP_PlayPawn.BP_PlayPawn_C|SetSelectedMesh _asbp_play_pawn 0))
    (Development|PrintString (Utilities|GetDisplayName _output_get))))

(event EventBeginPlay
  (bind _returnvalue (Components|GetOwner))
  (bind _returnvalue_2 (Actor|GetComponentbyClass _returnvalue "/Script/Engine.CapsuleComponent"))
  (Variables|Default|SetOwning%20Mesh (Actor|GetComponentbyClass _returnvalue "/Script/Engine.StaticMeshComponent"))
  (Collision|BindEventtoOnComponentBeginOverlap _returnvalue_2 (delegate Custom|On%20Begin%20Overlap))
  (Collision|BindEventtoOnComponentEndOverlap _returnvalue_2 (delegate Custom|On%20End%20Overlap)))