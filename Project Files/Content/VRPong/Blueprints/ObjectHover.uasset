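; ObjectHover is a component that makes its owning actor hover, bobbing up and down and swaying back and forth in yaw.
; Each Tick applies world offset and rotation deltas scaled by delta time and a shared TimeFactor.
; Separate accumulators flip the UpDown and LeftRight flags when their maximum travel is reached, producing linear back-and-forth motion.
; BeginPlay starts both accumulators at half range, centering the motion on the initial transform.
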(event EventTick
  (params (DeltaSeconds :type Float%20%28single-precision%29))
  (bind _time_factor (Variables|Default|GetTime%20Factor))
  (bind _returnvalue (* DeltaSeconds _time_factor))
  (Utilities|FlowControl|Sequence
    (:then_0
      (bind _output_get (Variables|Default|SetTemp%20Float _returnvalue))
      (if (Variables|Default|GetbUpDown)
        (Transformation|AddActorWorldOffset (Components|GetOwner) (Math|Vector|MakeVector 0.0 0.0 _output_get))
        (bind _output_get_2 (Variables|Default|SetCurrent%20Vertical%20Movement (+ (Variables|Default|GetCurrent%20Vertical%20Movement) (Math|Float|Absolute(Float) _output_get))))
        (if (>= _output_get_2 (Variables|Default|GetMax%20Vertical%20Movement))
          (Variables|Default|SetCurrent%20Vertical%20Movement 0.0)
          (Variables|Default|SetbUpDown false))
        (else
          (Math|Float|NegateFloat _output_get
            (:%20%20
              (Transformation|AddActorWorldOffset (Components|GetOwner) (Math|Vector|MakeVector 0.0 0.0 _output_get))
              (bind _output_get_3 (Variables|Default|SetCurrent%20Vertical%20Movement (+ (Variables|Default|GetCurrent%20Vertical%20Movement) (Math|Float|Absolute(Float) _output_get))))
              (if (>= _output_get_3 (Variables|Default|GetMax%20Vertical%20Movement))
                (Variables|Default|SetCurrent%20Vertical%20Movement 0.0)
                (Variables|Default|SetbUpDown true)))))))
    (:then_1
      (bind _output_get_4 (Variables|Default|SetTemp%20Float _returnvalue))
      (if (Variables|Default|GetbLeftRight)
        (Class|Actor|AddActorWorldRotation (Components|GetOwner) (Math|Rotator|MakeRotator 0.0 0.0 _output_get_4))
        (bind _output_get_5 (Variables|Default|SetCurrent%20Rotational%20Movement (+ (Variables|Default|GetCurrent%20Rotational%20Movement) (Math|Float|Absolute(Float) _output_get_4))))
        (if (>= _output_get_5 (Variables|Default|GetMax%20Rotational%20Movement))
          (Variables|Default|SetCurrent%20Rotational%20Movement 0.0)
          (Variables|Default|SetbLeftRight false))
        (else
          (Math|Float|NegateFloat _output_get_4
            (:%20%20
              (Class|Actor|AddActorWorldRotation (Components|GetOwner) (Math|Rotator|MakeRotator 0.0 0.0 _output_get_4))
              (bind _output_get_6 (Variables|Default|SetCurrent%20Rotational%20Movement (+ (Variables|Default|GetCurrent%20Rotational%20Movement) (Math|Float|Absolute(Float) _output_get_4))))
              (if (>= _output_get_6 (Variables|Default|GetMax%20Rotational%20Movement))
                (Variables|Default|SetCurrent%20Rotational%20Movement 0.0)
                (Variables|Default|SetbLeftRight true)))))))))

(event EventBeginPlay
  (Variables|Default|SetCurrent%20Vertical%20Movement (/ (Variables|Default|GetMax%20Vertical%20Movement) 2.0))
  (Variables|Default|SetCurrent%20Rotational%20Movement (/ (Variables|Default|GetMax%20Rotational%20Movement) 2.0)))