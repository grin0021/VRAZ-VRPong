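; BP_Confetti is a VR Pong actor that fires two confetti effects when it begins play, provided EnableConfetti is set.
; On BeginPlay it activates the Confetti1 and Confetti2 components, then moves each to world height zero while keeping its X and Y.
; Tick and Destroyed only call their parent events, and the construction script is empty.
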(event EventBeginPlay
  (bind _confetti1 (Variables|Default|GetConfetti1))
  (bind _confetti2 (Variables|Default|GetConfetti2))
  (bind _returnvalue (Transformation|GetWorldLocation _confetti2))
  (bind _returnvalue_2 (Transformation|GetWorldLocation _confetti1))
  (|CallParentFunction)
  (if (Variables|Default|GetbEnableConfetti)
    (Components|Activation|Activate _confetti1 false)
    (Transformation|SetWorldLocation _confetti1 (Math|Vector|MakeVector (.x _returnvalue_2) (.y _returnvalue_2) 0.0) false false)
    (Components|Activation|Activate _confetti2 false)
    (Transformation|SetWorldLocation _confetti2 (Math|Vector|MakeVector (.x _returnvalue) (.y _returnvalue) 0.0) false false)))

(event EventTick
  (params (DeltaSeconds :type Float%20%28single-precision%29))
  (|CallParentFunction DeltaSeconds))

(event EventDestroyed
  (|CallParentFunction))

(fn ConstructionScript)