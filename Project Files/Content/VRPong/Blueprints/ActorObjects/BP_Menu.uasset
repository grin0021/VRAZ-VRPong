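; BP_Menu is the VR Pong menu actor, hosting a widget that, unless static, is placed in front of the player and facing the camera on spawn.
; It moves the pawn's WidgetInteractionComponent to the right or left motion controller, where that hand's interact input switches hands or clicks.
; A Niagara laser tracks from the active controller to the hit point.
; The UI input mapping context lasts until destruction, and SetFirstMenu selects the WB_AllMenus page.
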(event Input|EnhancedActionEvents|EnhancedInputActionIA_Interact_Left
  (params (ActionValue :type Boolean) (ElapsedSeconds :type Float%20%28double-precision%29) (TriggeredSeconds :type Float%20%28double-precision%29) (InputAction :type Input%20Action%20Object%20Reference :default "/Game/VRPong/Input/Actions/IA_Interact_Left.IA_Interact_Left"))
  (bind _leftmotion (Variables|Default|GetLeftMotion))
  ;[1 1 1] Interaction between controllers and menu
  (:Started
    (if (== (Variables|Default|GetTrackedController) _leftmotion)
      (Class|WidgetInteractionComponent|PressPointerKey (Variables|Default|GetInteract%20ref) "LeftMouseButton")
      (else
        (bind _output_get (Variables|Default|SetTrackedController _leftmotion))
        (Transformation|AttachComponentToComponent (Variables|Default|GetInteract%20ref) _output_get "None" "SnapToTarget" "SnapToTarget" "KeepRelative" true))))
  (:Completed
    (Class|WidgetInteractionComponent|ReleasePointerKey (Variables|Default|GetInteract%20ref) "LeftMouseButton")))

(event Input|EnhancedActionEvents|EnhancedInputActionIA_Interact_Right
  (params (ActionValue :type Boolean) (ElapsedSeconds :type Float%20%28double-precision%29) (TriggeredSeconds :type Float%20%28double-precision%29) (InputAction :type Input%20Action%20Object%20Reference :default "/Game/VRPong/Input/Actions/IA_Interact_Right.IA_Interact_Right"))
  (bind _rightmotion (Variables|Default|GetRightMotion))
  ;[1 1 1] Interaction between controllers and menu
  (:Started
    (if (== (Variables|Default|GetTrackedController) _rightmotion)
      (Class|WidgetInteractionComponent|PressPointerKey (Variables|Default|GetInteract%20ref) "LeftMouseButton")
      (else
        (bind _output_get (Variables|Default|SetTrackedController _rightmotion))
        (Transformation|AttachComponentToComponent (Variables|Default|GetInteract%20ref) _output_get "None" "SnapToTarget" "SnapToTarget" "KeepRelative" true))))
  (:Completed
    (Class|WidgetInteractionComponent|ReleasePointerKey (Variables|Default|GetInteract%20ref) "LeftMouseButton")))

(event EventBeginPlay
  (bind _returnvalue (Game|GetPlayerController 0))
  (CallFunction|SetControllerReferences)
  (CallFunction|SetInteractionComponents)
  (Input|EnableInput _returnvalue)
  (Input|AddMappingContext (PlayerController|LocalPlayerSubsystems|GetEnhancedInputLocalPlayerSubsystem _returnvalue) "/Game/VRPong/Input/Contexts/IMC_UI.IMC_UI" 1 "(bIgnoreAllPressedKeysUntilRelease=True,bForceImmediately=False,bNotifyUserSettings=False)")
  (if (not (Variables|Default|GetbIsStatic))
    (Transformation|SetWorldLocation (Variables|Default|GetWidget) (+ (Camera|GetCameraLocation (Game|GetPlayerCameraManager 0)) (* (Transformation|GetActorForwardVector (Game|Player|GetPlayerPawn 0)) 1e+02)) false false)
    (Transformation|SetWorldRotation (Variables|Default|GetWidget) (Math|Rotator|FindLookatRotation (Transformation|GetWorldLocation (Variables|Default|GetWidget)) (Camera|GetCameraLocation (Game|GetPlayerCameraManager 0))) false false)
    (Transformation|SetRelativeScale3D (Variables|Default|GetWidget) "0.250000,0.250000,0.250000")))

(event EventDestroyed
  (Input|RemoveMappingContext (PlayerController|LocalPlayerSubsystems|GetEnhancedInputLocalPlayerSubsystem (Game|GetPlayerController 0)) "/Game/VRPong/Input/Contexts/IMC_UI.IMC_UI" "(bIgnoreAllPressedKeysUntilRelease=True,bForceImmediately=False,bNotifyUserSettings=False)"))

(event EventTick
  (params (DeltaSeconds :type Float%20%28single-precision%29))
  (bind _trackedcontroller (Variables|Default|GetTrackedController))
  (bind _interact_ref (Variables|Default|GetInteract%20ref))
  (bind _returnvalue (Transformation|GetWorldLocation _trackedcontroller))
  (bind (_returnvalue_hitcomponent _returnvalue_impactpoint) (|GetLastHitResult _interact_ref))
  (Utilities|FlowControl|Sequence
    (:then_0
      (Utilities|FlowControl|DoOnce false
        (:Completed
          (Rendering|SetVisibility (Variables|Default|GetLaser) true false))))
    (:then_1
      (Class|NiagaraDataInterfaceArrayFunctionLibrary|SetNiagaraArrayVectorValue (Variables|Default|GetLaser) "User.PointArray" 0 _returnvalue false)
      (Utilities|IsValid _returnvalue_hitcomponent
        (:Is%20Valid
          (Class|NiagaraDataInterfaceArrayFunctionLibrary|SetNiagaraArrayVectorValue (Variables|Default|GetLaser) "User.PointArray" 1 _returnvalue_impactpoint false))
        (:Is%20Not%20Valid
          (Class|NiagaraDataInterfaceArrayFunctionLibrary|SetNiagaraArrayVectorValue (Variables|Default|GetLaser) "User.PointArray" 1 (+ (* (Math|Vector|GetForwardVector _interact_ref) "100.000000,100.000000,100.000000") _returnvalue) false))))))

(fn ConstructionScript)

(fn SetInteractionComponents
  (bind _output_get (Variables|Default|SetInteract%20ref (Actor|GetComponentbyClass (Game|Player|GetPlayerPawn 0) "/Script/UMG.WidgetInteractionComponent")))
  (Transformation|AttachComponentToComponent _output_get (Variables|Default|GetTrackedController) "None" "SnapToTarget" "SnapToTarget" "KeepRelative" true))

(fn SetControllerReferences
  (bind _returnvalue (Game|GetPlayerCharacter 0))
  (bind _returnvalue_2 (Actor|GetComponentsByClass _returnvalue "/Script/HeadMountedDisplay.MotionControllerComponent"))
  (if (> (Utilities|Array|Length _returnvalue_2) 0)
    (bind _output_get (LocalVariables|SetLocal%20Motion%20Refs _returnvalue_2))
    (for _array_element _output_get
      (if (== (Variables|/Script/HeadMountedDisplay.MotionControllerComponent|GetMotionSource _array_element) "Right")
        (bind _output_get_2 (Variables|Default|SetRightMotion _array_element))
        (Variables|Default|SetTrackedController _output_get_2)
        (else
          (Variables|Default|SetLeftMotion _array_element))))))

(fn SetFirstMenu
  (params (InMenu :type String))
  (bind _aswb_all_menus (Utilities|Casting|CastToWB_AllMenus (UserInterface|GetWidget (Variables|Default|GetWidget))))
  (Default|SwitchMenuVisibility _aswb_all_menus 0 InMenu))