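; BP_Target is a target actor for VR Pong that shows a score display once it is flagged for death.
; While CuedForDeath is set, Tick reveals the ScoreDisplay widget component and pushes ActualScoreValue into its WB_TargetScoreDisplay every frame.
; SetMaterialColor creates dynamic material instances on two mesh slots and tints both green, dark yellow or red as the Factor argument rises.
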(event EventTick
  (params (DeltaSeconds :type Float%20%28single-precision%29))
  (bind _scoredisplay (Variables|Default|GetScoreDisplay))
  (if (Variables|Default|GetbCuedForDeath)
    (Rendering|SetVisibility _scoredisplay true false)
    (bind _aswb_target_score_display (Utilities|Casting|CastToWB_TargetScoreDisplay (UserInterface|GetWidget _scoredisplay)))
    (Default|SetScoreNumber _aswb_target_score_display (Variables|Default|GetactualScoreValue))))

(event EventSetMaterialColor
  (params (factor :type Float%20%28single-precision%29))
  (bind _returnvalue (Rendering|Material|CreateDynamicMaterialInstance (Variables|Default|GetStaticMesh) 1 "/Game/VRPong/ModelImports/Materials/Material_002.Material_002" "None" :!class /Script/Engine.PrimitiveComponent))
  (Variables|Default|SetElement1 _returnvalue)
  (bind _returnvalue_2 (Rendering|Material|CreateDynamicMaterialInstance (Variables|Default|GetStaticMesh) 2 "/Game/VRPong/ModelImports/Materials/Material_002.Material_002" "None" :!class /Script/Engine.PrimitiveComponent))
  (Variables|Default|SetElement2 _returnvalue_2)
  (if (<= factor 2.0)
    (Rendering|Material|SetVectorParameterValue (Variables|Default|GetElement1) "Color" (Utilities|Struct|MakeLinearColor 0.0 1.0 0.0 1.0) :!class /Script/Engine.MaterialInstanceDynamic)
    (Rendering|Material|SetVectorParameterValue (Variables|Default|GetElement2) "Color" (Utilities|Struct|MakeLinearColor 0.0 1.0 0.0 1.0) :!class /Script/Engine.MaterialInstanceDynamic)
    (elif (<= factor 4.0)
      (Rendering|Material|SetVectorParameterValue (Variables|Default|GetElement1) "Color" (Utilities|Struct|MakeLinearColor 0.5 0.5 0.0 1.0) :!class /Script/Engine.MaterialInstanceDynamic)
      (Rendering|Material|SetVectorParameterValue (Variables|Default|GetElement2) "Color" (Utilities|Struct|MakeLinearColor 0.5 0.5 0.0 1.0) :!class /Script/Engine.MaterialInstanceDynamic)
      (else
        (Rendering|Material|SetVectorParameterValue (Variables|Default|GetElement1) "Color" (Utilities|Struct|MakeLinearColor 1.0 0.0 0.0 1.0) :!class /Script/Engine.MaterialInstanceDynamic)
        (Rendering|Material|SetVectorParameterValue (Variables|Default|GetElement2) "Color" (Utilities|Struct|MakeLinearColor 1.0 0.0 0.0 1.0) :!class /Script/Engine.MaterialInstanceDynamic)))))

(fn ConstructionScript)