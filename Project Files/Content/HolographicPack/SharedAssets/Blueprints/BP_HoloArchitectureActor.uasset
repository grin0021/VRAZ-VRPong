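; Holographic architecture actor configured entirely in the construction script, with optional door and windows and a team index.
; TeamIndex is written to default custom primitive data slot 0 on every primitive under TeamIndexGrp.
; HasDoor and DoorLocked set visibility and collision on the locked and unlocked door groups, with the locked group updated inside the unlocked group's loop.
; HasWindows toggles window visibility, while window collision is always disabled.
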(event EventBeginPlay)

(event Collision|EventActorBeginOverlap
  (params (OtherActor :type Actor%20Object%20Reference)))

(event EventTick
  (params (DeltaSeconds :type Float%20%28single-precision%29)))

(fn ConstructionScript
  (bind _doorlockedgrp (Variables|Default|GetDoorLockedGrp))
  (bind _doorunlockedgrp (Variables|Default|GetDoorUnlockedGrp))
  (bind _windowgrp (Variables|Default|GetWindowGrp))
  (Utilities|FlowControl|Sequence
    (:then_0
      ;[1 1 1] Team Index
      (for _array_element (Components|GetChildrenComponents (Variables|Default|GetTeamIndexGrp) true)
        (bind _asprimitive_component (Utilities|Casting|CastToPrimitiveComponent _array_element))
        (Rendering|Material|SetDefaultCustomPrimitiveDataFloat _asprimitive_component 0 (Math|Conversions|ToFloat(Integer) (Variables|HolographicAssetValues|GetTeamIndex)))))
    (:then_1
      ;[1 1 1] Door
      ;;[1 1 1] Is door visible?
      (if (Variables|HolographicAssetValues|GetHasDoor)
        ;;[1 1 1] Is door locked?
        (if (Variables|HolographicAssetValues|GetDoorLocked)
          ;;[1 1 1] Unlocked Grp
          (Rendering|SetVisibility _doorunlockedgrp false true)
          (for _array_element_2 (Components|GetChildrenComponents _doorunlockedgrp true)
            (bind _asprimitive_component_2 (Utilities|Casting|CastToPrimitiveComponent _array_element_2))
            (Collision|SetCollisionEnabled _asprimitive_component_2 "NoCollision")
            ;;[1 1 1] Locked Grp
            (Rendering|SetVisibility _doorlockedgrp true true)
            (for _array_element_3 (Components|GetChildrenComponents _doorlockedgrp true)
              (bind _asprimitive_component_3 (Utilities|Casting|CastToPrimitiveComponent _array_element_3))
              (Collision|SetCollisionEnabled _asprimitive_component_3 "QueryAndPhysics")))
          (else
            (Rendering|SetVisibility _doorunlockedgrp true true)
            (for _array_element_4 (Components|GetChildrenComponents _doorunlockedgrp true)
              (bind _asprimitive_component_4 (Utilities|Casting|CastToPrimitiveComponent _array_element_4))
              (Collision|SetCollisionEnabled _asprimitive_component_4 "QueryAndPhysics")
              (Rendering|SetVisibility _doorlockedgrp false true)
              (for _array_element_5 (Components|GetChildrenComponents _doorlockedgrp true)
                (bind _asprimitive_component_5 (Utilities|Casting|CastToPrimitiveComponent _array_element_5))
                (Collision|SetCollisionEnabled _asprimitive_component_5 "NoCollision")))))
        (else
          (Rendering|SetVisibility _doorunlockedgrp false true)
          (for _array_element_6 (Components|GetChildrenComponents _doorunlockedgrp true)
            (bind _asprimitive_component_6 (Utilities|Casting|CastToPrimitiveComponent _array_element_6))
            (Collision|SetCollisionEnabled _asprimitive_component_6 "NoCollision")
            (Rendering|SetVisibility _doorlockedgrp false true)
            (for _array_element_7 (Components|GetChildrenComponents _doorlockedgrp true)
              (bind _asprimitive_component_7 (Utilities|Casting|CastToPrimitiveComponent _array_element_7))
              (Collision|SetCollisionEnabled _asprimitive_component_7 "NoCollision"))))))
    (:then_2
      ;[1 1 1] Windows
      (Rendering|SetVisibility _windowgrp (Variables|HolographicAssetValues|GetHasWindows) true)
      (for _array_element_8 (Components|GetChildrenComponents _windowgrp true)
        (bind _asprimitive_component_8 (Utilities|Casting|CastToPrimitiveComponent _array_element_8))
        (Collision|SetCollisionEnabled _asprimitive_component_8 "NoCollision")))))