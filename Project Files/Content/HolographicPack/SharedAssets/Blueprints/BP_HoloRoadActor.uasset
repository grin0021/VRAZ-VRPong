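; Holographic road actor that configures its team index and optional sidewalk meshes in the construction script, with no active runtime logic.
; TeamIndex is written to custom primitive data slot 0 on primitives under TeamIndexGrp and SidewalkGrp, presumably for materials to read.
; EnableSidewalkDisabled sets SidewalkGrp visibility, and those sidewalk primitives always have collision turned off.
; GetTeamPrimitiveComponents is an empty stub.
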(event EventBeginPlay)

(event Collision|EventActorBeginOverlap
  (params (OtherActor :type Actor%20Object%20Reference)))

(event EventTick
  (params (DeltaSeconds :type Float%20%28single-precision%29)))

(fn ConstructionScript
  (bind _sidewalkgrp (Variables|Default|GetSidewalkGrp))
  (Utilities|FlowControl|Sequence
    (:then_0
      ;[1 1 1] Team Index
      (for _array_element (Components|GetChildrenComponents (Variables|Default|GetTeamIndexGrp) true)
        (bind _asprimitive_component (Utilities|Casting|CastToPrimitiveComponent _array_element))
        (Rendering|Material|SetDefaultCustomPrimitiveDataFloat _asprimitive_component 0 (Math|Conversions|ToFloat(Integer) (Variables|HolographicAssetValues|GetTeamIndex)))))
    (:then_1
      ;[1 1 1] Sidewalk
      (Rendering|SetVisibility _sidewalkgrp (Variables|HolographicAssetValues|GetEnable%20Sidewalk%20%28disabled%29) true)
      (for _array_element_2 (Components|GetChildrenComponents _sidewalkgrp true)
        (bind _asprimitive_component_2 (Utilities|Casting|CastToPrimitiveComponent _array_element_2))
        (Collision|SetCollisionEnabled _asprimitive_component_2 "NoCollision")
        (Rendering|Material|SetDefaultCustomPrimitiveDataFloat _asprimitive_component_2 0 (Math|Conversions|ToFloat(Integer) (Variables|HolographicAssetValues|GetTeamIndex)))))))

(fn GetTeamPrimitiveComponents
  (return 0))