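; BP_HoloPropActor is a holographic prop actor configured at construction time by a team index and toggles for neon outline and lights.
; The construction script writes TeamIndex into custom primitive data slot 0 on primitive children of the team, neon outline and light groups.
; It also shows or hides the outline and light groups with propagation to children.
; Event graph nodes are disabled placeholders and GetTeamPrimitiveComponents is an empty stub.
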(event EventBeginPlay)

(event Collision|EventActorBeginOverlap
  (params (OtherActor :type Actor%20Object%20Reference)))

(event EventTick
  (params (DeltaSeconds :type Float%20%28single-precision%29)))

(fn ConstructionScript
  (bind _lightgrp (Variables|Default|GetLightGrp))
  (Utilities|FlowControl|Sequence
    (:then_0
      ;[1 1 1] Team Index
      (for _array_element (Components|GetChildrenComponents (Variables|Default|GetTeamIndexGrp) true)
        (bind _asprimitive_component (Utilities|Casting|CastToPrimitiveComponent _array_element))
        (Rendering|Material|SetDefaultCustomPrimitiveDataFloat _asprimitive_component 0 (Math|Conversions|ToFloat(Integer) (Variables|HolographicAssetValues|GetTeamIndex)))))
    (:then_1
      ;[1 1 1] Neon Outline
      (Rendering|SetVisibility (Variables|Default|GetNeonOutlineGrp) (Variables|HolographicAssetValues|GetEnableNeonOutline) true)
      (for _array_element_2 (Components|GetChildrenComponents (Variables|Default|GetNeonOutlineGrp) true)
        (bind _asprimitive_component_2 (Utilities|Casting|CastToPrimitiveComponent _array_element_2))
        (Rendering|Material|SetDefaultCustomPrimitiveDataFloat _asprimitive_component_2 0 (Math|Conversions|ToFloat(Integer) (Variables|HolographicAssetValues|GetTeamIndex)))))
    (:then_2
      ;[1 1 1] Lights
      (Rendering|SetVisibility _lightgrp (Variables|HolographicAssetValues|GetEnableLights) true)
      (for _array_element_3 (Components|GetChildrenComponents _lightgrp true)
        (bind _asprimitive_component_3 (Utilities|Casting|CastToPrimitiveComponent _array_element_3))
        (Rendering|Material|SetDefaultCustomPrimitiveDataFloat _asprimitive_component_3 0 (Math|Conversions|ToFloat(Integer) (Variables|HolographicAssetValues|GetTeamIndex)))))))

(fn GetTeamPrimitiveComponents
  (return 0))